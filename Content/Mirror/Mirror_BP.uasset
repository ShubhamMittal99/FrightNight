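; Mirror actor that the player aims with the arrow keys, taking input directly from player controller 0 on BeginPlay.
; Up and Down pitch MirrorMain, while Left and Right yaw MirrorFrame, both in local space.
; Each key opens a Gate while held, and Tick feeds all four through a Sequence.
; Rotation steps by Speed every frame without delta-time scaling, so turn rate depends on frame rate.
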(event `Key|Up`
  (params (Key :type "Key Structure"))
  (:`Pressed`
    (goto _label :!via `Open`))
  (:`Released`
    (goto _label :!via `Close`)))

(event `Key|Down`
  (params (Key :type "Key Structure"))
  (:`Pressed`
    (goto _label_2 :!via `Open`))
  (:`Released`
    (goto _label_2 :!via `Close`)))

(event `self.ReceiveTick`
  (params (DeltaSeconds :type "Float (single-precision)"))
  (bind _mirror_main (`self.Mirror_Main`))
  (bind _mirror_frame (`self.Mirror_Frame`))
  (bind _speed (`self.speed`))
  (bind _returnvalue (`KismetMathLibrary.MakeRotator` 0.0 0.0 _speed))
  (bind _returnvalue_2 (`KismetMathLibrary.MakeRotator` 0.0 _speed))
  (`|ExecutionSequence`
    (:`then_0`
      (`/Engine/EditorBlueprintResources/StandardMacros.Gate` true :!label _label
        (:`Exit`
          (`SceneComponent.K2_AddLocalRotation` _mirror_main (* _returnvalue_2 -1.0) false false))))
    (:`then_1`
      (`/Engine/EditorBlueprintResources/StandardMacros.Gate` true :!label _label_2
        (:`Exit`
          (`SceneComponent.K2_AddLocalRotation` _mirror_main _returnvalue_2 false false))))
    (:`then_2`
      (`/Engine/EditorBlueprintResources/StandardMacros.Gate` true :!label _label_3
        (:`Exit`
          (`SceneComponent.K2_AddLocalRotation` _mirror_frame (* _returnvalue -1.0) false false))))
    (:`then_3`
      (`/Engine/EditorBlueprintResources/StandardMacros.Gate` true :!label _label_4
        (:`Exit`
          (`SceneComponent.K2_AddLocalRotation` _mirror_frame _returnvalue false false))))))

(event `self.ReceiveBeginPlay`
  (`self.EnableInput` (`GameplayStatics.GetPlayerController` 0)))

(event `Key|Left`
  (params (Key :type "Key Structure"))
  (:`Pressed`
    (goto _label_3 :!via `Open`))
  (:`Released`
    (goto _label_3 :!via `Close`)))

(event `Key|Right`
  (params (Key :type "Key Structure"))
  (:`Pressed`
    (goto _label_4 :!via `Open`))
  (:`Released`
    (goto _label_4 :!via `Close`)))

(fn `UserConstructionScript`)