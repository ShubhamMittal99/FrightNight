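; BP_FNHUD is a HUD Blueprint that shows the player's on-screen interface and a centered crosshair.
; On BeginPlay it creates the HUD widget and adds it to the viewport.
; Each DrawHUD call draws the M_Crosshair material as a small fixed-size square, offset by half its size to sit at screen center.
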(event `self.ReceiveBeginPlay`
  (bind _returnvalue (`|CreateWidget` "/Game/StarterContent/Blueprints/UI/HUD.HUD_C"))
  (`UserWidget.AddToViewport` _returnvalue 0))

(event `self.ReceiveDrawHUD`
  (params (SizeX :type Integer) (SizeY :type Integer))
  (bind _returnvalue (/ 32.0 2.0))
  (`self.DrawMaterial` "/Game/Materials/M_Crosshair.M_Crosshair" (- (`KismetMathLibrary.Conv_IntToDouble` (/ SizeX 2)) _returnvalue) (- (`KismetMathLibrary.Conv_IntToDouble` (/ SizeY 2)) _returnvalue) 32.0 32.0 0.0 0.0 1.0 1.0))

(fn `UserConstructionScript`)